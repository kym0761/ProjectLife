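; BP_TeleportToBuilding_Test is a test trigger that moves a pawn entering its box to a Destination actor's location and rotation.
; After a successful teleport, only for a locally controlled pawn, it sets atmospheric fog and sky sphere visibility from the inverse of SkyOff.
; Both sky actors are looked up by class at that moment rather than referenced directly.
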(event `self.Box.OnComponentBeginOverlap`
  (params (OverlappedComponent :type "PrimitiveComponent Object Reference") (OtherActor :type "Actor Object Reference") (OtherComp :type "PrimitiveComponent Object Reference") (OtherBodyIndex :type Integer) (bFromSweep :type Boolean) (SweepResult :type "HitResult Structure (by ref)"))
  (bind _destination (`self.Destination`))
  (bind (_returnvalue_location _returnvalue_rotation) (`KismetMathLibrary.BreakTransform` (`self.GetTransform` _destination)))
  (bind _aspawn (cast `Pawn` OtherActor))
  (`/Engine/EditorBlueprintResources/StandardMacros.IsValid` _destination
    (:`Is Valid`
      (bind _returnvalue (`self.K2_TeleportTo` _aspawn _returnvalue_location _returnvalue_rotation))
      (if _returnvalue
        (if (`Pawn.IsLocallyControlled` _aspawn)
          (bind _returnvalue_2 (`GameplayStatics.GetActorOfClass` "/Script/Engine.AtmosphericFog"))
          (`SceneComponent.SetVisibility` (`AtmosphericFog.AtmosphericFogComponent` _returnvalue_2) (not (`self.bSkyOff`)) false)
          (bind _returnvalue_3 (`GameplayStatics.GetActorOfClass` "/Engine/EngineSky/BP_Sky_Sphere.BP_Sky_Sphere_C"))
          (`SceneComponent.SetVisibility` (`/Engine/EngineSky/BP_Sky_Sphere.SkySphereMesh` _returnvalue_3) (not (`self.bSkyOff`)) false))))))

(fn `UserConstructionScript`)