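; Test actor that turns Niagara particle callback data into radial damage.
; It registers itself as the system's export callback through a user variable and reactivates the Niagara effect on a looping five-second timer.
; Each exported particle's Size acts as a switch: positive deals a large blast at the actor's location with a debug sphere, otherwise small damage lands at the particle's position.
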(event `self.ReceiveBeginPlay`
  (`NiagaraComponent.SetNiagaraVariableObject` (`self.Niagara`) "User.BP_Callback" self)
  (`KismetSystemLibrary.K2_SetTimerDelegate` (delegate `커스텀이벤트_0`) 5.0 true))

(event `커스텀이벤트_0`
  (`ActorComponent.Activate` (`self.Niagara`) true))

(event `self.ReceiveParticleData`
  (params (Data :type "Array of BasicParticleData Structure (by ref)") (NiagaraSystem :type "NiagaraSystem Object Reference"))
  (bind _returnvalue (`self.K2_GetActorLocation`))
  ;[1 1 1] Interface : Niagara Particle Callback Handler
  (for _array_element Data
    (bind (_position _size) (break `BasicParticleData` _array_element))
    (if (> _size 0.0)
      (`KismetSystemLibrary.DrawDebugSphere` _returnvalue 100.0 12 (struct :`R` 0.257525 :`G` 0.509261 :`B` 0.541667 :`A` 1.0) 1.0 1.0)
      (`GameplayStatics.ApplyRadialDamage` :`BaseDamage` 50.0 :`Origin` _returnvalue :`DamageRadius` 100.0 :`DamageCauser` null :`InstigatedByController` null)
      (else
        (`GameplayStatics.ApplyRadialDamage` :`BaseDamage` 2.0 :`Origin` _position :`DamageRadius` 5.0 :`DamageCauser` null :`InstigatedByController` null)))))

(fn `UserConstructionScript`)