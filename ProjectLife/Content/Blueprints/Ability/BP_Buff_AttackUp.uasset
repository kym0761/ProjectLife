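; Attack-up buff ability that raises its owner's attack coefficient while it lasts.
; The passive effect casts the owner to BasicCharacter and adds a fixed amount to AttackCoefficient on its StatComponent, and EndAbility subtracts the same amount.
; The active effect is a placeholder that only prints a Korean debug question about what should happen when attack first rises, and the end effect is empty.
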(event `self.ActivateActiveEffect`
  (`KismetSystemLibrary.PrintString` "공격력이 최초에 올랐을 땐 무엇을 해야하는지?"))

(event `self.ActivatePassiveEffect`
  (bind _asbasic_character (cast `BasicCharacter` (`self.AbilityOwner`)))
  (bind _statcomponent (`BasicCharacter.StatComponent` _asbasic_character))
  (set `StatComponent.AttackCoefficient` (+ (`StatComponent.AttackCoefficient` _statcomponent) 1.0) _statcomponent))

(event `self.EndAbility`
  (bind _asbasic_character (cast `BasicCharacter` (`self.AbilityOwner`)))
  (bind _statcomponent (`BasicCharacter.StatComponent` _asbasic_character))
  (set `StatComponent.AttackCoefficient` (- (`StatComponent.AttackCoefficient` _statcomponent) 1.0) _statcomponent))

(event `self.ActivateEndEffect`)

(fn `UserConstructionScript`)