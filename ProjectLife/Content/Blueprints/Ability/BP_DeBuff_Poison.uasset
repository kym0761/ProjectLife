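; Poison debuff ability that deals periodic damage to the actor that owns it.
; On active effect it targets the owner and starts a looping one-second timer, which applies damage from the first effect amount in the ability data while the target is valid.
; Ending the ability clears the timer.
; Passive and end effects are placeholders that print Korean design notes proposing an added slow and finishing damage.
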(event `self.ActivateActiveEffect`
  (set `self.AbilityTarget` (`self.AbilityOwner`))
  (bind _returnvalue (`KismetSystemLibrary.K2_SetTimerDelegate` (delegate `Poison to Owner`) 1.0 true))
  (set `self.PoisonTimer` _returnvalue))

(event `Poison to Owner`
  (bind _abilitytarget (`self.AbilityTarget`))
  (`/Engine/EditorBlueprintResources/StandardMacros.IsValid` _abilitytarget
    (:`Is Valid`
      (`GameplayStatics.ApplyDamage` _abilitytarget (`|GetArrayItem` (`.AbilityEffectAmounts` (break `AbilityDataStruct` (`self.AbilityData`)))) null self))))

(event `self.ActivatePassiveEffect`
  (`KismetSystemLibrary.PrintString` "독에 걸리면 슬로우가 추가로 걸린다면 좋을 듯?"))

(event `self.EndAbility`
  (bind _poisontimer (`self.PoisonTimer`))
  (if (`KismetSystemLibrary.K2_IsTimerActiveHandle` _poisontimer)
    (`KismetSystemLibrary.K2_ClearAndInvalidateTimerHandle` _poisontimer)))

(event `self.ActivateEndEffect`
  (`KismetSystemLibrary.PrintString` "독이 끝나면 끝맛나는 딜이 더 들어간다?"))

(fn `UserConstructionScript`)