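; Shield ability that grants its owning BasicCharacter bonus Shield on the StatComponent.
; Activation adds the first AbilityData effect amount; ending subtracts ShieldAmount from the stat, clamped at zero or above.
; TakeDamageHandle drains ShieldAmount and destroys the ability without its end effect when depleted, but a TODO notes it still needs hooking to owner damage.
; Passive and end effects only print design ideas.
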(event `self.ActivateActiveEffect`
  (bind _asbasic_character (cast `BasicCharacter` (`self.AbilityOwner`)))
  (bind _statcomponent (`BasicCharacter.StatComponent` _asbasic_character))
  (`/Engine/EditorBlueprintResources/StandardMacros.IsValid` _statcomponent
    (:`Is Valid`
      (set `StatComponent.Shield` (+ (`StatComponent.Shield` _statcomponent) (`|GetArrayItem` (`.AbilityEffectAmounts` (break `AbilityDataStruct` (`self.AbilityData`))))) _statcomponent))))

(event `self.ActivatePassiveEffect`
  (`KismetSystemLibrary.PrintString` "실드가 생기면 방어력이 올랐으면 좋겠다."))

(event `Take Damage Handle`
  (params (Damage :type "Float (double-precision)"))
  ;[1 1 1] TODO : 실드가 데미지를 받았을 때 발동할 효과를 위해서,
  ;  Ablity Owner의 Take Damage 등에
  ; 연결할 방법을 모색해야함.
  (bind _output_get (set `self.ShieldAmount` (- (`self.ShieldAmount`) Damage)))
  (if (<= _output_get 0.0)
    (`self.DestroyAbilityWithoutEndEffect`)))

(event `self.EndAbility`
  (bind _asbasic_character (cast `BasicCharacter` (`self.AbilityOwner`)))
  (bind _statcomponent (`BasicCharacter.StatComponent` _asbasic_character))
  (`/Engine/EditorBlueprintResources/StandardMacros.IsValid` _statcomponent
    (:`Is Valid`
      (set `StatComponent.Shield` (`KismetMathLibrary.FClamp` (- (`StatComponent.Shield` _statcomponent) (`self.ShieldAmount`)) 0.0 10000000.0) _statcomponent))))

(event `self.ActivateEndEffect`
  (`KismetSystemLibrary.PrintString` "실드가 깨지면 주위에 폭파 데미지?"))

(fn `UserConstructionScript`)