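; BP_QuestGiver is an interactable quest giver that offers quests to players through an approval popup.
; Interact shows a temporary approval widget to the interactor's PlayerController, passing the interactor as receiver and itself as owner.
; GiveQuest checks for a player-controlled accepter and a valid class, then calls AddQuest on the project GameInstance, printing failures.
; Both the class check and AddQuest have no quest wired in.
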(event `self.Interact`
  (params (InteractCauser :type "Pawn Object Reference"))
  (bind `_as플레이어_컨트롤러` (cast `PlayerController` (`Pawn.GetController` InteractCauser)))
  (bind _returnvalue (`|CreateWidget` "/Game/Blueprints/Quest/UI_QuestApproval_Temp.UI_QuestApproval_Temp_C" `_as플레이어_컨트롤러` InteractCauser self))
  (`UserWidget.AddToViewport` _returnvalue 0))

(event `Give Quest`
  (params (QuestAccepter :type "Pawn Object Reference"))
  (if (`Pawn.IsPlayerControlled` QuestAccepter)
    (bind _asproject_life_game_instance (cast `ProjectLIfeGameInstance` (`GameplayStatics.GetGameInstance`))
      (:`then`
        (if (`KismetSystemLibrary.IsValidClass` null)
          (`ProjectLIfeGameInstance.AddQuest` _asproject_life_game_instance "")
          (else
            (`KismetSystemLibrary.PrintString` "Quest Not Valid"))))
      (:`CastFailed`
        (`KismetSystemLibrary.PrintString` "Failed Game instance cast")))
    (else
      (`KismetSystemLibrary.PrintString` "Not Player"))))

(fn `UserConstructionScript`)