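; BP_Cow is an interactable cow animal that shows a heart when the interaction succeeds.
; Interact checks InteractOK, calls the parent's interaction, then shows HeartWidget while a timeline animates its relative Z location, hiding it when finished.
; The construction script is empty; logic for randomly picking one of three material variants for two mesh slots is left disconnected and never runs.
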(event `self.Interact`
  (params (InteractCauser :type "Pawn Object Reference"))
  (if (`self.bInteractOK`)
    (`parent.Interact` InteractCauser)
    (`SceneComponent.SetVisibility` (`self.HeartWidget`) true false)
    (bind (_direction `_새_트랙_0`) (`Timeline|타임라인_0` :!via `PlayFromStart`)
      (:`Update`
        (`SceneComponent.K2_SetRelativeLocation` (`self.HeartWidget`) (`KismetMathLibrary.MakeVector` 0.0 0.0 `_새_트랙_0`) false false))
      (:`Finished`
        (`SceneComponent.SetVisibility` (`self.HeartWidget`) false false)))))

(fn `UserConstructionScript`
  (locals (`Material Index` :type Integer :default 0)))