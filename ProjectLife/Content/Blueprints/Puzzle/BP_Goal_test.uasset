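; BP_Goal_test is a puzzle goal actor that plays a short finishing sequence and quits the game.
; Its overlap event accepts a valid, controlled BasicCharacter, then after a brief delay disables its input and starts a looping timer that makes it jump repeatedly.
; An extremely low spring arm camera lag speed all but stops the camera following, then the screen fades out before the game exits.
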(event `self.ReceiveBeginPlay`
  (add `self.OnActorBeginOverlap` (delegate `OnGoal`)))

(event `OnGoal` :!signature `self.OnActorBeginOverlap`
  (params (OverlappedActor :type "Actor Object Reference") (OtherActor :type "Actor Object Reference"))
  (`/Engine/EditorBlueprintResources/StandardMacros.IsValid` OtherActor
    (:`Is Valid`
      (bind _output_get (set `self.Overlapped Actor` OtherActor))
      (if (`KismetMathLibrary.ClassIsChildOf` (`GameplayStatics.GetObjectClass` _output_get) "/Script/ProjectLife.BasicCharacter")
        (bind `_as캐릭터` (cast `Character` (`self.Overlapped Actor`)))
        (if (`Pawn.IsControlled` `_as캐릭터`)
          (`KismetSystemLibrary.Delay` 0.15)
          (`self.DisableInput` `_as캐릭터` null)
          (`KismetSystemLibrary.K2_SetTimerDelegate` (delegate `Auto Jumping`) 0.5 true)
          (bind _asbp_basic_character (cast `/Game/Blueprints/BP_BasicCharacter` `_as캐릭터`))
          (bind _springarm (`BasicCharacter.SpringArm` _asbp_basic_character))
          (set `SpringArmComponent.CameraLagSpeed` 0.001 _springarm)
          (set `SpringArmComponent.bEnableCameraLag` true _springarm)
          (`KismetSystemLibrary.Delay` 0.5)
          (`PlayerCameraManager.StartCameraFade` :`self` (`GameplayStatics.GetPlayerCameraManager` 0) :`ToAlpha` 1.0 :`Duration` 2.0 :`bHoldWhenFinished` true)
          (`KismetSystemLibrary.Delay` 2.5)
          (`KismetSystemLibrary.QuitGame` null "Quit"))))))

(event `Auto Jumping`
  (`Character.Jump` (stale `OnGoal` `_as캐릭터`)))

(fn `UserConstructionScript`)