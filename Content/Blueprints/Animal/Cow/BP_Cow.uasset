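; Cow animal Blueprint that reacts to player interaction with a heart popup and varies its look per instance.
; When interaction is allowed, Interact runs the parent logic, then shows HeartWidget, animates its relative Z height with a timeline and hides it on finish.
; The construction script picks one of three random indices to set a paired material on both mesh slots, re-rolling whenever construction reruns.
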(event `self.Interact`
  (params (InteractCauser :type "Pawn Object Reference"))
  (if (`self.bInteractOK`)
    (`parent.Interact` InteractCauser)
    (`SceneComponent.SetVisibility` (`self.HeartWidget`) true false)
    (bind (_direction `_새_트랙_0`) (`Timeline|타임라인_0` :!via `PlayFromStart`)
      (:`Update`
        (`SceneComponent.K2_SetRelativeLocation` (`self.HeartWidget`) (`KismetMathLibrary.MakeVector` 0.0 0.0 `_새_트랙_0`) false false))
      (:`Finished`
        (`SceneComponent.SetVisibility` (`self.HeartWidget`) false false)))))

(fn `UserConstructionScript`
  (locals (`Material Index` :type Integer :default 0))
  (bind _mesh (`self.Mesh`))
  (bind _output_get (set `local.Material Index` (`KismetMathLibrary.RandomIntegerInRange` 0 2)))
  (`PrimitiveComponent.SetMaterial` _mesh 0 (`|GetArrayItem` (`self.Material1`) _output_get))
  (`PrimitiveComponent.SetMaterial` _mesh 1 (`|GetArrayItem` (`self.Material2`) _output_get)))