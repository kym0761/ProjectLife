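; BP_Cow is a cow animal that plays a random sound when interacted with and varies its appearance.
; Interact spawns a random entry from Sounds attached to the capsule, gated by a DoOnce that resets when the audio finishes, so sounds do not overlap.
; The construction script picks one random index to set a matching pair of materials on the mesh's two slots.
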(event `self.Interact`
  (params (InteractCauser :type "Pawn Object Reference"))
  (bind _sounds (`self.Sounds`))
  (`/Engine/EditorBlueprintResources/StandardMacros.DoOnce` false :!label _label
    (:`Completed`
      (bind _returnvalue (`GameplayStatics.SpawnSoundAttached` (`|GetArrayItem` _sounds (`KismetMathLibrary.RandomIntegerInRange` 0 (`KismetArrayLibrary.Array_LastIndex` _sounds))) (`self.CapsuleComponent`) "None" (0.0 0.0 0.0) (struct) "KeepRelativeOffset" false 1.0 1.0 0.0 null null))
      (add `AudioComponent.OnAudioFinished` _returnvalue (delegate `Reset`)))))

(event `Reset`
  (goto _label :!via `Reset`))

(fn `UserConstructionScript`
  (locals (`Material Index` :type Integer :default 0))
  (bind _mesh (`self.Mesh`))
  (bind _output_get (set `local.Material Index` (`KismetMathLibrary.RandomIntegerInRange` 0 2)))
  (`PrimitiveComponent.SetMaterial` _mesh 0 (`|GetArrayItem` (`self.Material1`) _output_get))
  (`PrimitiveComponent.SetMaterial` _mesh 1 (`|GetArrayItem` (`self.Material2`) _output_get)))