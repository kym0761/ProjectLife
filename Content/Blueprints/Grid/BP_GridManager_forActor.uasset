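; Grid manager actor that spawns and tracks an X-by-Y grid of actors of a configurable class.
; SpawnGridActor clears the previous grid, then spawns actors at fixed 50-unit spacing from the manager's location, ignoring its rotation, and stores them in GridArr.
; It does nothing when both dimensions are zero or less.
; RemoveAllGridActors destroys the stored actors and empties the array; the construction script is empty.
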(fn `Remove All Grid Actors`
  (for _array_element (`self.GridArr`)
    (`/Engine/EditorBlueprintResources/StandardMacros.IsValid` _array_element
      (:`Is Valid`
        (`self.K2_DestroyActor` _array_element))))
  (`KismetArrayLibrary.Array_Clear` (`self.GridArr`)))

(fn `SpawnGridActor`
  (bind (_returnvalue_x _returnvalue_y _returnvalue_z) (`KismetMathLibrary.BreakVector` (`self.K2_GetActorLocation`)))
  (if (not (and (<= (`self.X`) 0) (<= (`self.Y`) 0)))
    (for _array_element (`self.GridArr`)
      (`/Engine/EditorBlueprintResources/StandardMacros.IsValid` _array_element
        (:`Is Valid`
          (`self.K2_DestroyActor` _array_element))))
    (`KismetArrayLibrary.Array_Clear` (`self.GridArr`))
    (for _index (range (`self.X`))
      (for _index_2 (range (`self.Y`))
        (bind _returnvalue (`|SpawnActorFromClass` (`self.Class`) (`KismetMathLibrary.MakeTransform` (`KismetMathLibrary.MakeVector` (+ (* _index 50.0) _returnvalue_x) (+ (* _index_2 50.0) _returnvalue_y) _returnvalue_z)) "Undefined" "OverrideRootScale" null null))
        (`KismetArrayLibrary.Array_Add` (`self.GridArr`) _returnvalue)))))

(fn `UserConstructionScript`)