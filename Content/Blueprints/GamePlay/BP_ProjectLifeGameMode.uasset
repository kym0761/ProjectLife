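; Game mode Blueprint for ProjectLife that advances the in-game clock.
; On BeginPlay it caches the ProjectLifeGameState and starts a fast looping timer.
; Each tick of that timer fires IncreaseHour, which, despite its name, adds a five-minute increment to the game state's InGameTime through the game-time addition helper.
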(event `self.ReceiveBeginPlay`
  (`parent.ReceiveBeginPlay`)
  (bind _asproject_life_game_state (cast `ProjectLifeGameState` (`GameplayStatics.GetGameState`)))
  (set `self.As Project Life Game State` _asproject_life_game_state)
  (`KismetSystemLibrary.K2_SetTimerDelegate` (delegate `Increase Hour`) 0.05 true))

(event `Increase Hour`
  (bind _as_project_life_game_state (`self.As Project Life Game State`))
  (`/Engine/EditorBlueprintResources/StandardMacros.IsValid` _as_project_life_game_state
    (:`Is Valid`
      (set `ProjectLifeGameState.InGameTime` (`GameTimeFunctionLibrary.Plus_GameTimeGameTime` (`ProjectLifeGameState.InGameTime` _as_project_life_game_state) (make `InGameTime` 0 0 0 0 5)) _as_project_life_game_state))))

(fn `UserConstructionScript`)