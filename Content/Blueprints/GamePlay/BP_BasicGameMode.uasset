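; BP_BasicGameMode is the game mode that drives the in-game clock.
; On BeginPlay it casts the game instance to BP_ProjectLifeGameInstance and caches it, then starts a looping half-second timer.
; Each timer tick adds one in-game hour to the GameTime stored on the game instance, using a custom game-time addition function.
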(event `self.ReceiveBeginPlay`
  (`parent.ReceiveBeginPlay`)
  (bind _asbp_project_life_game_instance (cast `/Game/Blueprints/GamePlay/BP_ProjectLifeGameInstance` (`GameplayStatics.GetGameInstance`)))
  (set `self.As BP Project Life Game Instance` _asbp_project_life_game_instance)
  (`KismetSystemLibrary.K2_SetTimerDelegate` (delegate `Increase Hour`) 0.5 true))

(event `Increase Hour`
  (bind _as_bp_project_life_game_instance (`self.As BP Project Life Game Instance`))
  (set `ProjectLIfeGameInstance.GameTime` (`GameTimeFunctionLibrary.Plus_GameTimeGameTime` (`ProjectLIfeGameInstance.GameTime` _as_bp_project_life_game_instance) (make `InGameTime` 0 0 0 1)) _as_bp_project_life_game_instance))

(fn `UserConstructionScript`)