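; Basic character Blueprint that sets up the player HUD and carries debug keys for testing the calendar, quest and ability systems.
; BeginPlay adds the HP/shield widget and a hidden quest view; keys show quests, toggle the calendar, advance the game mode's day or spawn and start a random buff.
; Interact shows a placeholder speech bubble.
; AnyDamage calls its parent, then temporarily forwards damage to the first shield in AbilityComponent's map.
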(event `Key|K`
  (params (Key :type "Key Structure"))
  ;[1 1 1] Calendar Testing
  (:`Pressed`
    (bind _asbp_basic_game_mode (cast `/Game/Blueprints/GameMode/BP_BasicGameMode` (`GameplayStatics.GetGameMode`)))
    (`BasicGameMode.IncreaseDay` _asbp_basic_game_mode 1)))

(event `Key|Q`
  (params (Key :type "Key Structure"))
  (bind _questviewref (`self.QuestViewRef`))
  ;[1 1 1] Quest Test
  (:`Pressed`
    (`/Engine/EditorBlueprintResources/StandardMacros.IsValid` _questviewref
      (:`Is Valid`
        (`/Game/Blueprints/Quest/Widget_QuestView.ShowQuestView` _questviewref)))))

(event `Key|L`
  (params (Key :type "Key Structure"))
  ;[1 1 1] Calendar Testing
  (:`Pressed`
    (`/Engine/EditorBlueprintResources/StandardMacros.IsValid` (`self.CalendarRef`)
      (:`Is Valid`
        (`Widget.RemoveFromParent` (`self.CalendarRef`))
        (set `self.CalendarRef` null))
      (:`Is Not Valid`
        (bind _asplayer_controller (cast `PlayerController` (`self.GetController`)))
        (bind _returnvalue (`|CreateWidget` "/Game/UI/Widget/WBP_CalendarWidget.WBP_CalendarWidget_C" _asplayer_controller))
        (`UserWidget.AddToViewport` _returnvalue 0)
        (set `self.CalendarRef` _returnvalue)))))

(event `self.ReceiveBeginPlay`
  (bind _asplayer_controller (cast `PlayerController` (`self.GetController`)))
  (bind _returnvalue (`|CreateWidget` "/Game/Blueprints/Ability/Widget_HPandShield.Widget_HPandShield_C" _asplayer_controller))
  (`UserWidget.AddToViewport` _returnvalue 0)
  (bind _returnvalue_2 (`|CreateWidget` "/Game/Blueprints/Quest/Widget_QuestView.Widget_QuestView_C" _asplayer_controller))
  (set `self.QuestViewRef` _returnvalue_2)
  (`UserWidget.AddToViewport` _returnvalue_2 0)
  (`Widget.SetVisibility` _returnvalue_2 "Hidden"))

(event `self.Interact`
  (params (InteractCauser :type "Pawn Object Reference"))
  (bind _speechbubblewidget (`self.SpeechBubbleWidget`))
  (`SceneComponent.SetVisibility` _speechbubblewidget true false)
  (`SceneComponent.SetHiddenInGame` _speechbubblewidget false false)
  (`SpeechWidgetComponent.SpeechTrigger` _speechbubblewidget "hello hello hello \nhello  hello \nhellohellohellohello")
  (`KismetSystemLibrary.PrintString` "Interact to Character is Success"))

(event `Key|B`
  (params (Key :type "Key Structure"))
  (bind _buffarray (`self.BuffArray`))
  ;[1 1 1] Random Ability Test
  (:`Pressed`
    (bind _returnvalue (`|SpawnActorFromClass` (`|GetArrayItem` _buffarray (`KismetMathLibrary.RandomIntegerInRange` 0 (`KismetArrayLibrary.Array_LastIndex` _buffarray))) (`KismetMathLibrary.MakeTransform` (0.0 0.0 0.0)) "Undefined" "OverrideRootScale" self null))
    (set `Ability.AbilityOwner` self _returnvalue)
    (`Ability.StartAbility` _returnvalue)))

(event `self.ReceiveAnyDamage`
  (params (Damage :type "Float (single-precision)") (DamageType :type "DamageType Object Reference") (InstigatedBy :type "Controller Object Reference") (DamageCauser :type "Actor Object Reference"))
  ;[1 1 1] temporal Function For shield BP's Damage Handle
  (`parent.ReceiveAnyDamage` Damage DamageType InstigatedBy DamageCauser)
  (bind _values (`BlueprintMapLibrary.Map_Values` (`AbilityComponent.AbilityMap` (`self.AbilityComponent`))))
  (for _array_element _values
    (bind _asbp_shield (cast `/Game/Blueprints/Ability/BP_Shield` _array_element))
    (`/Game/Blueprints/Ability/BP_Shield.Take Damage Handle` _asbp_shield Damage)
    (break)))

(fn `UserConstructionScript`)