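; BP_Buff_AttackUp is a buff ability that raises the owning BasicCharacter's attack while it is active.
; ActivateAbility casts the owner to BasicCharacter and adds a fixed amount to AttackCoefficient on its StatComponent.
; EndAbility subtracts the same amount, so the change is additive and does not cache the original value.
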(event `self.ActivateAbility`
  (bind _asbasic_character (cast `BasicCharacter` (`self.GetOwner`)))
  (bind _statcomponent (`BasicCharacter.StatComponent` _asbasic_character))
  (set `StatComponent.AttackCoefficient` (+ (`StatComponent.AttackCoefficient` _statcomponent) 1.0) _statcomponent))

(event `self.EndAbility`
  (bind _asbasic_character (cast `BasicCharacter` (`self.GetOwner`)))
  (bind _statcomponent (`BasicCharacter.StatComponent` _asbasic_character))
  (set `StatComponent.AttackCoefficient` (- (`StatComponent.AttackCoefficient` _statcomponent) 1.0) _statcomponent))

(fn `UserConstructionScript`)