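; BP_Shield is a buff actor that grants a shield to its owning BasicCharacter.
; PlayBuff adds ShieldAmount to the Shield value on the character's Stat.
; TakeDamageHandle drains its own ShieldAmount by incoming damage and destroys the actor once it is used up.
; EndBuff subtracts whatever ShieldAmount remains from the character's Shield, clamped so it cannot go below zero.
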(event `self.PlayBuff`
  (bind _asbasic_character (cast `BasicCharacter` (`self.GetOwner`)))
  (bind _stat (`BasicCharacter.Stat` _asbasic_character))
  (`/Engine/EditorBlueprintResources/StandardMacros.IsValid` _stat
    (:`Is Valid`
      (set `StatComponent.Shield` (+ (`StatComponent.Shield` _stat) (`self.ShieldAmount`)) _stat))))

(event `Take Damage Handle`
  (params (Damage :type "Float (double-precision)"))
  (bind _output_get (set `self.ShieldAmount` (- (`self.ShieldAmount`) Damage)))
  (if (<= _output_get 0.0)
    (`self.K2_DestroyActor`)))

(event `self.EndBuff`
  (bind _asbasic_character (cast `BasicCharacter` (`self.GetOwner`)))
  (bind _stat (`BasicCharacter.Stat` _asbasic_character))
  (`/Engine/EditorBlueprintResources/StandardMacros.IsValid` _stat
    (:`Is Valid`
      (set `StatComponent.Shield` (`KismetMathLibrary.FClamp` (- (`StatComponent.Shield` _stat) (`self.ShieldAmount`)) 0.0 10000000.0) _stat))))

(fn `UserConstructionScript`)