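; BP_Heal is a healing ability that periodically heals the BP_BasicCharacter that owns it.
; Activating the active effect starts a looping one-second timer that heals the owner by the first effect amount in AbilityData, and ending the ability clears that timer.
; The passive effect is a placeholder that only prints a Korean note wishing for increased speed during healing, and the end effect is empty.
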(event `self.ActivateActiveEffect`
  (bind _returnvalue (`KismetSystemLibrary.K2_SetTimerDelegate` (delegate `Heal to Owner`) 1.0 true))
  (set `self.HealTimer` _returnvalue))

(event `Heal to Owner`
  (bind _abilityowner (`self.AbilityOwner`))
  (`/Engine/EditorBlueprintResources/StandardMacros.IsValid` _abilityowner
    (:`Is Valid`
      (bind _asbp_basic_character (cast `/Game/Blueprints/BP_BasicCharacter` _abilityowner))
      (`ItemFunctionLibrary.Heal` _asbp_basic_character (`.AbilityEffectAmount1` (break `AbilityDataStruct` (`self.AbilityData`)))))))

(event `self.ActivatePassiveEffect`
  (`KismetSystemLibrary.PrintString` "힐을 받는 동안 스피드가 올랐으면 좋겠다"))

(event `self.EndAbility`
  (bind _healtimer (`self.HealTimer`))
  (if (`KismetSystemLibrary.K2_IsTimerActiveHandle` _healtimer)
    (`KismetSystemLibrary.K2_ClearAndInvalidateTimerHandle` _healtimer)))

(event `self.ActivateEndEffect`)

(fn `UserConstructionScript`)