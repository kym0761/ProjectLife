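; BP_AbilityPlayTrigger_Test is a test trigger volume that plays a configured ability on actors that walk into it.
; On BeginPlay, a text render shows the display name of the AbilityRef class.
; When an actor with an AbilityComponent overlaps the box, it spawns AbilityRef at the trigger's transform, sets that actor as owner and starts the ability.
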(event `self.ReceiveBeginPlay`
  (bind _abilityref (`self.AbilityRef`))
  (if (`KismetSystemLibrary.IsValidClass` _abilityref)
    (`TextRenderComponent.K2_SetText` (`self.TextRender`) (`KismetTextLibrary.Conv_StringToText` (`KismetSystemLibrary.GetClassDisplayName` _abilityref)))))

(event `self.Box.OnComponentBeginOverlap`
  (params (OverlappedComponent :type "PrimitiveComponent Object Reference") (OtherActor :type "Actor Object Reference") (OtherComp :type "PrimitiveComponent Object Reference") (OtherBodyIndex :type Integer) (bFromSweep :type Boolean) (SweepResult :type "HitResult Structure (by ref)"))
  (bind _abilityref (`self.AbilityRef`))
  (`/Engine/EditorBlueprintResources/StandardMacros.IsValid` OtherActor
    (:`Is Valid`
      (`/Engine/EditorBlueprintResources/StandardMacros.IsValid` (`self.GetComponentByClass` OtherActor "/Script/ProjectLife.AbilityComponent")
        (:`Is Valid`
          (if (`KismetSystemLibrary.IsValidClass` _abilityref)
            (bind _returnvalue (`|SpawnActorFromClass` _abilityref (`self.GetTransform`) "Undefined" "OverrideRootScale" null null))
            (`Ability.SetAbilityOwner` _returnvalue OtherActor)
            (`Ability.StartAbility` _returnvalue)))))))

(fn `UserConstructionScript`)