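; Quest giver actor that offers a quest to an interacting player and can register it in the game.
; Interact opens a temporary approval widget for the causer's player controller, passing the causer as receiver and itself as owner.
; A separate GiveQuest event checks that the accepter is player controlled, then adds the QuestToGive class to the ProjectLIfe game instance.
; Failed checks in GiveQuest print debug messages.
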(event `self.Interact`
  (params (InteractCauser :type "Pawn Object Reference"))
  (bind _asplayer_controller (cast `PlayerController` (`Pawn.GetController` InteractCauser)))
  (bind _returnvalue (`|CreateWidget` "/Game/Blueprints/Quest/QuestApproval_Temp.QuestApproval_Temp_C" _asplayer_controller InteractCauser self))
  (`UserWidget.AddToViewport` _returnvalue 0))

(event `Give Quest`
  (params (QuestAccepter :type "Pawn Object Reference"))
  (bind _questtogive (`self.QuestToGive`))
  (if (`Pawn.IsPlayerControlled` QuestAccepter)
    (bind _asproject_life_game_instance (cast `ProjectLIfeGameInstance` (`GameplayStatics.GetGameInstance`))
      (:`then`
        (if (`KismetSystemLibrary.IsValidClass` _questtogive)
          (`ProjectLIfeGameInstance.AddQuest` _asproject_life_game_instance _questtogive)
          (else
            (`KismetSystemLibrary.PrintString` "Quest Not Valid"))))
      (:`CastFailed`
        (`KismetSystemLibrary.PrintString` "Failed Game instance cast")))
    (else
      (`KismetSystemLibrary.PrintString` "Not Player"))))

(fn `UserConstructionScript`)