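; BP_SeedTest is a test seed item that plants a crop when used by a character.
; UseItem casts the owner to BP_BasicCharacter and asks it for an interactee, which must be a GridComponent.
; On success it spawns BP_CropTest at that component's world location and returns true.
; A failed cast returns false, and each outcome prints a debug string.
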(fn `UseItem`
  (returns (ReturnValue :type Boolean))
  (bind _asbp_basic_character (cast `/Game/Blueprints/BP_BasicCharacter` (`self.GetOwner`))
    (:`then`
      (bind _returnvalue (`BasicCharacter.FindInteractee` _asbp_basic_character))
      (bind _asgrid_component (cast `GridComponent` _returnvalue)
        (:`then`
          (`|SpawnActorFromClass` "/Game/Blueprints/Farming/BP_CropTest.BP_CropTest_C" (`KismetMathLibrary.Conv_VectorToTransform` (`SceneComponent.K2_GetComponentLocation` _asgrid_component)) "Undefined" "OverrideRootScale" null null)
          (`KismetSystemLibrary.PrintString` "OK")
          (return true))
        (:`CastFailed`
          (`KismetSystemLibrary.PrintString` "Can't Find GridComp"))))
    (:`CastFailed`
      (`KismetSystemLibrary.PrintString` "Owner is not Character")))
  (return false))

(fn `UserConstructionScript`)