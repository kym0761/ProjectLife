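; BP_CropTest is a test crop actor that turns into a harvested crop item when its GiveHarvest event is called.
; GiveHarvest spawns a BP_CropHarvested at a randomized offset above and around the crop, adjusting for collision but always spawning, then destroys the crop.
; The construction script is empty, and nothing in this graph calls the event or handles growth.
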(event `self.GiveHarvest`
  (`|SpawnActorFromClass` "/Game/Blueprints/Farming/BP_CropHarvested.BP_CropHarvested_C" (`KismetMathLibrary.MakeTransform` (`KismetMathLibrary.MakeVector` (+ (.x (`self.K2_GetActorLocation`)) (`KismetMathLibrary.RandomFloatInRange` -50.0 50.0)) (+ (.y (`self.K2_GetActorLocation`)) (`KismetMathLibrary.RandomFloatInRange` -50.0 50.0)) (+ (.z (`self.K2_GetActorLocation`)) (`KismetMathLibrary.RandomFloatInRange` 100.0 200.0)))) "AdjustIfPossibleButAlwaysSpawn" "OverrideRootScale" null null)
  (`self.K2_DestroyActor`))

(fn `UserConstructionScript`)