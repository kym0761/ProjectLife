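; BP_Item_Seed is a seed item that plants a crop on the farming grid cell detected by the player's character.
; SetSeed calls UseItem, which reaches the character through the owning player controller and asks its GridDetectComponent for a grid.
; On an empty grid it spawns BP_Crop, cross-links crop and grid, then destroys itself.
; An occupied grid only prints a message and returns false.
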(event `Set Seed`
  (`self.UseItem`))

(fn `UseItem`
  (returns (ReturnValue :type Boolean))
  (bind _returnvalue (`self.GetOwner`))
  (bind _asbp_basic_player_controller (cast `/Game/Blueprints/BP_BasicPlayerController` _returnvalue))
  (bind _asbp_basic_character (cast `/Game/Blueprints/BP_BasicCharacter` (`Controller.K2_GetPawn` _asbp_basic_player_controller))
    (:`then`
      (bind _returnvalue_2 (`GridDetectComponent.DetectGrid` (`BasicCharacter.GridDetectComponent` _asbp_basic_character)))
      (`/Engine/EditorBlueprintResources/StandardMacros.IsValid` _returnvalue_2
        (:`Is Valid`
          (`/Engine/EditorBlueprintResources/StandardMacros.IsValid` (`GridActor.Occupying` _returnvalue_2)
            (:`Is Valid`
              (`KismetSystemLibrary.PrintString` "Already Something Exist.")
              (return false))
            (:`Is Not Valid`
              (bind _returnvalue_3 (`|SpawnActorFromClass` "/Game/Blueprints/Farming/BP_Crop.BP_Crop_C" (`KismetMathLibrary.Conv_VectorToTransform` (`SceneComponent.K2_GetComponentLocation` (`Actor.RootComponent` _returnvalue_2))) "Undefined" "OverrideRootScale" null null))
              (`GridActor.SetOccupying` _returnvalue_2 _returnvalue_3)
              (set `Crop.GridRef` _returnvalue_2 _returnvalue_3)
              (`self.K2_DestroyActor`)
              (return true))))))
    (:`CastFailed`
      (`KismetSystemLibrary.PrintString` "Owner is not Character")
      (`KismetSystemLibrary.PrintString` (`KismetSystemLibrary.GetObjectName` _returnvalue))
      (return false))))

(fn `UserConstructionScript`)