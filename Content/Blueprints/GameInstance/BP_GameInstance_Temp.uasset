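; Game instance Blueprint that keeps the player's active and cleared quest lists.
; AddQuest appends a valid quest unless one of the same class is already active, in which case it prints a message.
; HandleQuestClear finds the active quest by class and moves it to ClearedQuests, using a stored index that this graph never resets between calls.
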(event `AddQuest`
  (params (InQuest :type "QuestBase Object Reference"))
  (`/Engine/EditorBlueprintResources/StandardMacros.IsValid` InQuest
    (:`Is Valid`
      (set `self.bCanAdd` true)
      (for _array_element (`self.Quests`)
        (if (== (`GameplayStatics.GetObjectClass` _array_element) (`GameplayStatics.GetObjectClass` InQuest))
          (set `self.bCanAdd` false)))
      (if (`self.bCanAdd`)
        (`KismetArrayLibrary.Array_Add` (`self.Quests`) InQuest)
        (else
          (`KismetSystemLibrary.PrintString` "Already Has This Quest"))))))

(event `Handle Quest Clear`
  (params (ClearedQuest :type "QuestBase Object Reference"))
  (bind _output (`|GetArrayItem` (`self.Quests`) (`self.Cleared Quest Index`)))
  (for (_array_element _array_index) (`self.Quests`)
    (if (== (`GameplayStatics.GetObjectClass` _array_element) (`GameplayStatics.GetObjectClass` ClearedQuest))
      (set `self.Cleared Quest Index` _array_index)))
  (if (>= (`self.Cleared Quest Index`) 0)
    (`/Engine/EditorBlueprintResources/StandardMacros.IsValid` _output
      (:`Is Valid`
        (`KismetArrayLibrary.Array_Add` (`self.ClearedQuests`) _output)
        (`KismetArrayLibrary.Array_Remove` (`self.Quests`) (`self.Cleared Quest Index`))))))