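; Attack-up buff that temporarily raises the attack coefficient of its owning BasicCharacter.
; PlayBuff adds BuffData.BuffAmount to the owner's Stat.AttackCoefficient, and EndBuff subtracts it again.
; Both events cast the owner to BasicCharacter and do nothing if the cast fails; duration and timing are not handled in this graph.
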(event `self.PlayBuff`
  (bind _asbasic_character (cast `BasicCharacter` (`self.GetOwner`)))
  (bind _stat (`BasicCharacter.Stat` _asbasic_character))
  (set `StatComponent.AttackCoefficient` (+ (`StatComponent.AttackCoefficient` _stat) (`.BuffAmount` (break `BuffDataStruct` (`self.BuffData`)))) _stat))

(event `self.EndBuff`
  (bind _asbasic_character (cast `BasicCharacter` (`self.GetOwner`)))
  (bind _stat (`BasicCharacter.Stat` _asbasic_character))
  (set `StatComponent.AttackCoefficient` (- (`StatComponent.AttackCoefficient` _stat) (`.BuffAmount` (break `BuffDataStruct` (`self.BuffData`)))) _stat))

(fn `UserConstructionScript`)