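; BP_DeBuff_Poison is a poison debuff that deals damage over time to its owner.
; PlayDeBuff starts a looping one-second timer whose tick applies DeBuffData's DeBuffAmount as damage to the owner, if valid.
; The instigator's controller is credited as event instigator and the debuff itself as damage causer.
; EndDeBuff clears the timer if it is still active.
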(event `self.PlayDeBuff`
  (bind _returnvalue (`KismetSystemLibrary.K2_SetTimerDelegate` (delegate `Poison to Owner`) 1.0 true))
  (set `self.PoisonTimer` _returnvalue))

(event `Poison to Owner`
  (bind _returnvalue (`self.GetOwner`))
  (`/Engine/EditorBlueprintResources/StandardMacros.IsValid` _returnvalue
    (:`Is Valid`
      (`GameplayStatics.ApplyDamage` _returnvalue (`.DeBuffAmount` (break `DeBuffDataStruct` (`self.DeBuffData`))) (`Pawn.GetController` (`self.GetInstigator`)) self))))

(event `self.EndDeBuff`
  (bind _poisontimer (`self.PoisonTimer`))
  (if (`KismetSystemLibrary.K2_IsTimerActiveHandle` _poisontimer)
    (`KismetSystemLibrary.K2_ClearAndInvalidateTimerHandle` _poisontimer)))

(fn `UserConstructionScript`)