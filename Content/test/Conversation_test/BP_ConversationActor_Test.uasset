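; Test conversation actor that opens a dialogue widget when a player-controlled causer interacts with it.
; Interact sets the Interacted flag, then ConversationStart creates WBP_Conversation with a back-reference to the actor, initializes it with InConversations and pauses the game.
; WhenConversationFinished unpauses the game and starts a short one-shot timer that resets Interacted, though this graph never checks that flag.
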(event `self.Interact`
  (params (InteractCauser :type "Pawn Object Reference"))
  (if (`self.IsPlayerControlled` InteractCauser)
    (set `self.bInteracted` true)
    (`self.Conversation Start`)))

(event `Conversation Start`
  (bind _returnvalue (`|CreateWidget` "/Game/UI/Widget/Conversation/WBP_Conversation.WBP_Conversation_C" (`GameplayStatics.GetPlayerController` 0)))
  (set `/Game/UI/Widget/Conversation/WBP_Conversation.NPC_Ref` self _returnvalue)
  (`UserWidget.AddToViewport` _returnvalue 0)
  (`ConversationWidget.InitConversationWidget` _returnvalue (`self.In Conversations`))
  (`GameplayStatics.SetGamePaused` true))

(event `When Conversation Finished`
  (`KismetSystemLibrary.K2_SetTimerDelegate` (delegate `커스텀이벤트_0`) 5.0)
  (`GameplayStatics.SetGamePaused` false))

(event `커스텀이벤트_0`
  (set `self.bInteracted` false))

(fn `UserConstructionScript`)