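; Test character that walks an AI-driven route to a destination route node when play begins.
; On BeginPlay it picks the RouteNode whose display name is BP_RouteNode_Dest and asks RouteFind for a route to it.
; MoveToDest then runs AI Move To on each actor in the result, advancing the index and calling itself when a move finishes, until an entry is invalid.
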(event `self.ReceiveBeginPlay`
  (bind _destination (`self.Destination`))
  ;[1 1 1] Find Destination
  (bind _outactors (`GameplayStatics.GetAllActorsOfClass` "/Script/ProjectLife.RouteNode"))
  (for _array_element _outactors
    (if (`KismetStringLibrary.EqualEqual_StrStr` (`KismetSystemLibrary.GetDisplayName` _array_element) "BP_RouteNode_Dest")
      (set `self.Destination` _array_element)))
  (`/Engine/EditorBlueprintResources/StandardMacros.IsValid` _destination
    (:`Is Valid`
      (bind _returnvalue (`RouteFindComponent.FindRoute` (`self.RouteFind`) _destination))
      (set `self.Result` _returnvalue)
      (set `self.i` 0)
      (`self.Move to Dest`))))

(event `Move to Dest`
  (bind _output (`|GetArrayItem` (`self.Result`) (`self.i`)))
  (`/Engine/EditorBlueprintResources/StandardMacros.IsValid` _output
    (:`Is Valid`
      (`AITask_MoveTo.AIMoveTo` (cast `AIController` (`self.GetController`) :!pure true) (0.0 0.0 0.0) _output
        (:`OnMoveFinished`
          (`/Engine/EditorBlueprintResources/StandardMacros.IncrementInt` (`self.i`)
            (:`  `
              (`self.Move to Dest`))))))))

(fn `UserConstructionScript`)